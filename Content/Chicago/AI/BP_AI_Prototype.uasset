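; BP_AI_Prototype is a prototype AI combatant that registers itself with the CombatBrainSubsystem on BeginPlay.
; At startup it creates a dynamic material instance on its Cylinder mesh, stores it as MatIns and sets its Color parameter to red.
; Unconnected nodes that would set green or blue never run, and the construction script is empty.
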(event `self.ReceiveBeginPlay`
  (bind _cylinder (`self.Cylinder`))
  (bind _returnvalue (`PrimitiveComponent.CreateDynamicMaterialInstance` _cylinder 0 (`PrimitiveComponent.GetMaterial` _cylinder 0) "None"))
  (bind _output_get (set `self.MatIns` _returnvalue))
  (`MaterialInstanceDynamic.SetVectorParameterValue` _output_get "Color" (struct :`R` 1.0 :`B` 0.010856 :`A` 1.0))
  (`CombatBrainSubsystem.RegisterCombatant` (subsystem `CombatBrainSubsystem`) self))

(fn `UserConstructionScript`)